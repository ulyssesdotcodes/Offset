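; Player controller that toggles an offset teleport, leaving a shadow character at the player's original spot.
; Pressing Offset spawns the shadow, then moves the player to the cursor or touch hit point, raised by a ground height traced at BeginPlay.
; Each tick the shadow copies the player's transform, minus the stored offset, and velocity.
; Pressing again sweeps the player to the shadow's location and destroys it.
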(event EventTick
  (params (DeltaSeconds :type Float%20%28single-precision%29))
  (if (Variables|Default|GetShadowExists)
    (CallFunction|ShadowEventTick)))

(event EventBeginPlay
  ;[1 1 1] Get offset from ground to use later
  (Utilities|GetZOffset))

(event Input|ActionEvents|InputActionOffset
  (:Pressed
    (if (Variables|Default|GetShadowExists)
      (CallFunction|ReturntoShadow)
      (else
        (CallFunction|CreateShadowCharacter)
        (CallFunction|OffsetCharacter)))))

(fn ConstructionScript)

(fn OffsetCharacter
  (bind (_hitresult _returnvalue) (Game|Player|GetHitResultUnderCursorbyChannel "TraceTypeQuery1" true))
  (bind (_hitresult_2 _returnvalue_2) (Class|PlayerController|GetHitResultUnderFingerbyChannel "Touch1" "TraceTypeQuery1" true))
  (bind _actortransform (Utilities|GetPlayerTransform))
  (bind _zoffset (Variables|Default|GetZOffset))
  (bind _location (Collision|BreakHitResult _hitresult))
  (bind _location_2 (Collision|BreakHitResult _hitresult_2))
  (bind _location_3 (Math|Transform|BreakTransform _actortransform))
  (bind (_x _y _z) (Math|Vector|BreakVector _location_3))
  (bind _returnvalue_3 (+ _location _location_2))
  (bind (_x_2 _y_2 _z_2) (Math|Vector|BreakVector _returnvalue_3))
  (bind _returnvalue_4 (- _x_2 _x))
  (bind _returnvalue_5 (- _y_2 _y))
  (bind _returnvalue_6 (+ _zoffset _z_2))
  (bind _returnvalue_7 (- _returnvalue_6 _z))
  (bind _returnvalue_8 (Math|Vector|MakeVector _returnvalue_4 _returnvalue_5 _returnvalue_7))
  (if (or _returnvalue _returnvalue_2)
    (Variables|Default|SetOffset _returnvalue_8)
    (Transformation|SetActorLocation (Game|GetPlayerCharacter 0) (+ _returnvalue_8 _location_3) false)))

(fn CreateShadowCharacter
  (bind _returnvalue (Game|SpawnActorfromClass "/Game/Blueprints/ShadowCharacter.ShadowCharacter_C" (Utilities|GetPlayerTransform) false))
  (Variables|Default|SetShadowCharacter _returnvalue)
  (Variables|Default|SetShadowExists true)
  (return false))

(fn ShadowEventTick
  (bind _actortransform (Utilities|GetPlayerTransform))
  (bind _shadowcharacter (Variables|Default|GetShadowCharacter))
  (bind (_location _rotation _scale) (Math|Transform|BreakTransform _actortransform))
  (Transformation|SetActorTransform _shadowcharacter (Math|Transform|MakeTransform (- _location (Variables|Default|GetOffset)) _rotation _scale))
  (Variables|/Script/Engine.MovementComponent|SetVelocity (Pawn|GetMovementComponent _shadowcharacter) (Variables|/Script/Engine.MovementComponent|GetVelocity (Pawn|GetMovementComponent (Game|GetPlayerCharacter 0))))
  (return))

(fn ReturntoShadow
  (bind _shadowcharacter (Variables|Default|GetShadowCharacter))
  (Variables|Default|SetShadowExists false)
  (Transformation|SetActorLocation (Game|GetPlayerCharacter 0) (Transformation|GetActorLocation _shadowcharacter) true)
  (Actor|DestroyActor _shadowcharacter)
  (return))